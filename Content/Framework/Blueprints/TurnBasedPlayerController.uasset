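; Player controller for a turn-based multiplayer game that tracks whether it is the local player's turn.
; On BeginPlay, a local controller creates the turn-based HUD and broadcasts the initial turn state.
; Client StartTurn and EndTurn events update IsMyTurn through SetMyTurn, which fires the OnMyTurnChanged dispatcher.
; A server EndTurn event asks the TurnBasedGameMode to cycle turns.
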(event `self.ReceiveBeginPlay`
  ;[1 1 1] Create the HUD once the game starts
  (if (`self.IsLocalController`)
    (bind _returnvalue (`|CreateWidget` "/Game/Framework/UserInterface/HUD_TurnBased.HUD_TurnBased_C" self))
    (`UserWidget.AddToViewport` _returnvalue 0)
    (`self.SetMyTurn` (`self.IsMyTurn`))))

(event `Start Turn (Client)`
  (`self.SetMyTurn` true))

(event `End Turn (Client)`
  (`self.SetMyTurn` false))

(event `End Turn (Server)`
  (`/Game/Framework/Blueprints/TurnBasedGameMode.Cycle Turns` (`self.GetTurnBasedGameMode`)))

(fn `SetMyTurn`
  (params (IsMyTurn :type Boolean))
  ;[1 1 1] Update the variable and call the event dispatcher
  (bind _output_get (set `self.IsMyTurn` IsMyTurn))
  (`self.OnMyTurnChanged` _output_get))

(fn `UserConstructionScript`)