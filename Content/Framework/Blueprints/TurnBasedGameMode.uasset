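; Turn-based game mode that runs player turns in a fixed order, starting once the desired player count joins and matches the PlayerOrder length.
; The current turn index maps through PlayerOrder to a TurnBasedPlayerController, which receives client start and end turn calls.
; Cycling ends the current turn, advances the index with modulo wraparound, and starts the next.
; Each turn start copies the active player's name to TurnBasedGameState.
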(event `self.K2_PostLogin`
  (params (NewPlayer :type "PlayerController Object Reference"))
  (bind _desirednumplayers (`self.DesiredNumPlayers`))
  ;[1 1 1] Start the game if the number of desired players joined and the order is given
  (bind _returnvalue (`self.GetNumPlayers`))
  (if (and (== _returnvalue _desirednumplayers) (== _desirednumplayers (`KismetArrayLibrary.Array_Length` (`self.PlayerOrder`))))
    (`self.Start Next Turn`)))

(event `Start Next Turn`
  (bind _player_controller (`self.GetCurrentPlayer`))
  ;[1 1 1] Start the turn for the next player
  (`/Game/Framework/Blueprints/TurnBasedPlayerController.Start Turn (Client)` _player_controller)
  (bind _asturn_based_game_state (cast `/Game/Framework/Blueprints/TurnBasedGameState` (`GameplayStatics.GetGameState`)))
  (bind _asturn_based_player_state (cast `/Game/Framework/Blueprints/TurnBasedPlayerState` (`Controller.PlayerState` _player_controller)))
  (set `/Game/Framework/Blueprints/TurnBasedGameState.CurrentPlayerName` (`/Game/Framework/Blueprints/TurnBasedPlayerState.PlayerName` _asturn_based_player_state) _asturn_based_game_state))

(event `Cycle Turns`
  ;[1 1 1] Cycle the turns by ending the turn for the current player and starting it for the next one
  (`/Game/Framework/Blueprints/TurnBasedPlayerController.End Turn (Client)` (`self.GetCurrentPlayer`))
  (set `self.CurrentPlayerIndex` (mod (+ (`self.CurrentPlayerIndex`) 1) (`self.NumPlayers`)))
  (`self.Start Next Turn`))

(fn `UserConstructionScript`)